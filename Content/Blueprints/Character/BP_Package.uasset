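; Delivery package that travels in an arc between an NPC and the player's hoverbike on pickup and drop-off.
; Pickup and DropOff disable bike movement, reshape a spline with a raised midpoint and play the shared MoveBox timeline.
; The timeline moves the cube along it, tracking the destination component's position.
; On finish it restores movement, then attaches to the bike or, after drop-off, calls Delivered and destroys itself.
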(event `Pickup`
  (params (NPC_Loc :type "Vector Structure"))
  (bind _returnvalue (`GameplayStatics.GetPlayerPawn` 0))
  (bind _spline (`self.Spline`))
  (bind _cube (`self.Cube`))
  (bind _returnvalue_2 (`self.K2_GetActorLocation` _returnvalue))
  (bind _asbp_hoverbike (cast `/Game/Blueprints/Character/BP_Hoverbike` (`GameplayStatics.GetPlayerPawn` 0) :!pure true))
  (bind _asbp_hoverbike_2 (cast `/Game/Blueprints/Character/BP_Hoverbike` _returnvalue :!pure true))
  (set `/Game/Blueprints/Character/BP_Hoverbike.CanMove` false _asbp_hoverbike_2)
  (set `self.DestComp` (`/Game/Blueprints/Character/BP_Hoverbike.PackagePosition` _asbp_hoverbike_2))
  (`SplineComponent.SetLocationAtSplinePoint` (`self.Spline`) 2 _returnvalue_2 "World" true)
  (`SplineComponent.SetLocationAtSplinePoint` (`self.Spline`) 1 (+ (`KismetMathLibrary.VLerp` NPC_Loc _returnvalue_2 0.5) (0.0 0.0 50.0)) "World" true)
  (bind (_direction _alpha) (`Timeline|MoveBox` :!via `PlayFromStart` :!label _label)
    (:`Update`
      (`SplineComponent.SetLocationAtSplinePoint` (`self.Spline`) 2 (`SceneComponent.K2_GetComponentLocation` (`self.DestComp`)) "World" true)
      (`SceneComponent.K2_SetWorldLocation` (`self.Cube`) (`SplineComponent.GetLocationAtDistanceAlongSpline` _spline (`KismetMathLibrary.Lerp` 0.0 (`SplineComponent.GetSplineLength` _spline) _alpha) "World") false false))
    (:`Finished`
      (`SceneComponent.K2_SetWorldLocation` _cube (`SceneComponent.K2_GetComponentLocation` (`self.DestComp`)) false false)
      (`SceneComponent.K2_SetWorldLocation` (`self.Spline`) (`SceneComponent.K2_GetComponentLocation` (`self.DestComp`)) false false)
      (`SceneComponent.K2_SetWorldRotation` _cube (`KismetMathLibrary.Conv_VectorToRotator` (`self.GetActorForwardVector` (cast `/Game/Blueprints/Character/BP_Hoverbike` (`GameplayStatics.GetPlayerPawn` 0) :!pure true))) false false)
      (set `/Game/Blueprints/Character/BP_Hoverbike.CanMove` true _asbp_hoverbike)
      (if (`self.DroppedOff`)
        (`/Game/Blueprints/Character/BP_Hoverbike.Delivered` (cast `/Game/Blueprints/Character/BP_Hoverbike` (`GameplayStatics.GetPlayerPawn` 0) :!pure true))
        (`self.K2_DestroyActor`)
        (else
          (`self.K2_AttachToComponent` (`/Game/Blueprints/Character/BP_Hoverbike.PackagePosition` _asbp_hoverbike) "None" "KeepWorld" "KeepWorld" "KeepWorld"))))))

(event `DropOff`
  (params (`NPC Loc` :type "SceneComponent Object Reference"))
  (bind _returnvalue (`SceneComponent.K2_GetComponentLocation` `NPC Loc`))
  (set `/Game/Blueprints/Character/BP_Hoverbike.CanMove` false (cast `/Game/Blueprints/Character/BP_Hoverbike` (`GameplayStatics.GetPlayerPawn` 0) :!pure true))
  (set `self.DestComp` `NPC Loc`)
  (`SplineComponent.SetLocationAtSplinePoint` (`self.Spline`) 2 _returnvalue "World" true)
  (`SplineComponent.SetLocationAtSplinePoint` (`self.Spline`) 1 (+ (`KismetMathLibrary.VLerp` (`SceneComponent.K2_GetComponentLocation` (`self.Cube`)) _returnvalue 0.5) (0.0 0.0 50.0)) "World" true)
  (set `self.DroppedOff` true)
  (goto _label :!via `PlayFromStart`))

(fn `UserConstructionScript`)