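; BP_Hoverbike is a player-driven, physics-based hoverbike with drive, turn, crouch and reset inputs.
; Input axes apply force and torque to the skeletal mesh, while four corner hover components receive crouch toggles.
; Each tick eases the visual mesh and its anim instance toward the turn lean, toggles line trails by speed, and pushes the bike down when airborne.
; Reset teleports it to a fixed height, keeping only yaw.
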(event `InputAxis|MoveForward`
  (params (AxisValue :type "Float (single-precision)"))
  ;[1 1 1] Turning
  (`PrimitiveComponent.AddForce` (`self.BikeSkMesh`) (* (`self.GetActorForwardVector`) (* (`self.ForwardForce`) AxisValue)) "None" false))

(event `InputAction|Reset`
  (params (Key :type "Key Structure"))
  ;[1 1 1] Reset Bike
  (:`Pressed`
    (`self.ResetBike`)))

(event `ResetBike`
  (bind (_returnvalue_x _returnvalue_y) (`KismetMathLibrary.BreakVector` (`self.K2_GetActorLocation`)))
  ;[1 1 1] Reset Bike
  (`self.K2_SetActorTransform` (`KismetMathLibrary.MakeTransform` (`KismetMathLibrary.MakeVector` _returnvalue_x _returnvalue_y 150.0) (`KismetMathLibrary.MakeRotator` 0.0 0.0 (.yaw (`self.K2_GetActorRotation`)))) false true))

(event `InputAxis|TurnRight`
  (params (AxisValue :type "Float (single-precision)"))
  ;[1 1 1] Turning
  (`PrimitiveComponent.AddTorqueInDegrees` (`self.BikeSkMesh`) (* (`self.GetActorUpVector`) (* (`self.TurnTorque`) AxisValue)) "None" false)
  (set `self.LeanAmount` (* AxisValue (`self.LeanDegrees`))))

(event `InputAction|Crouch`
  (params (Key :type "Key Structure"))
  (bind _bp_hovercomponentfr (`self.BP_HoverComponentFR`))
  ;[1 1 1] Crouching
  (:`Pressed`
    (`/Game/Blueprints/Character/BP_HoverComponent.Crouching` _bp_hovercomponentfr true)
    (`/Game/Blueprints/Character/BP_HoverComponent.Crouching` (`self.BP_HoverComponentBL`) true)
    (`/Game/Blueprints/Character/BP_HoverComponent.Crouching` (`self.BP_HoverComponentBR`) true)
    (`/Game/Blueprints/Character/BP_HoverComponent.Crouching` (`self.BP_HoverComponentFL`) true))
  (:`Released`
    (`/Game/Blueprints/Character/BP_HoverComponent.Crouching` _bp_hovercomponentfr false)
    (`/Game/Blueprints/Character/BP_HoverComponent.Crouching` (`self.BP_HoverComponentBL`) false)
    (`/Game/Blueprints/Character/BP_HoverComponent.Crouching` (`self.BP_HoverComponentBR`) false)
    (`/Game/Blueprints/Character/BP_HoverComponent.Crouching` (`self.BP_HoverComponentFL`) false)))

(event `self.ReceiveTick`
  (params (DeltaSeconds :type "Float (single-precision)"))
  (`self.SetBikeLean`)
  (`self.SetBikeTrails`)
  (`self.GroundingBike`))

(fn `GroundingBike`
  (bind _output_get (set `self.IsUpInAir` (and (not (`/Game/Blueprints/Character/BP_HoverComponent.Touching` (`self.BP_HoverComponentFR`))) (not (`/Game/Blueprints/Character/BP_HoverComponent.Touching` (`self.BP_HoverComponentBL`))) (not (`/Game/Blueprints/Character/BP_HoverComponent.Touching` (`self.BP_HoverComponentBR`))) (not (`/Game/Blueprints/Character/BP_HoverComponent.Touching` (`self.BP_HoverComponentFL`))))))
  (if _output_get
    (`PrimitiveComponent.AddForce` (`self.BikeSkMesh`) (* (0.0 0.0 -1.0) (`self.GroundingForce`)) "None" false) ; Attempt to ground
  ))

(fn `SetBikeLean`
  (bind _returnvalue (`KismetMathLibrary.MakeRotator` (`KismetMathLibrary.FInterpTo` (.roll (`SceneComponent.RelativeRotation` (`self.BikeVisualMesh`))) (`self.LeanAmount`) (`GameplayStatics.GetWorldDeltaSeconds`) 5.0)))
  (`SceneComponent.K2_SetRelativeRotation` (`self.BikeVisualMesh`) _returnvalue false false)
  (set `/Game/Blueprints/Anims/BP_AnimHoverBike.RotationValue` _returnvalue (cast `/Game/Blueprints/Anims/BP_AnimHoverBike` (`SkeletalMeshComponent.GetAnimInstance` (`self.BikeVisualMesh`)) :!pure true)))

(fn `SetBikeTrails`
  (bind _linesright (`self.LinesRight`))
  (bind _returnvalue (`PrimitiveComponent.GetPhysicsLinearVelocity` (`self.BikeSkMesh`) "None"))
  (if (<= (`KismetMathLibrary.VSize` _returnvalue) 500.0)
    (`ActorComponent.Deactivate` _linesright)
    (`ActorComponent.Deactivate` (`self.LinesLeft`))
    (`ActorComponent.Deactivate` (`self.LinesBrake`))
    (else
      (`ActorComponent.Activate` _linesright false)
      (`ActorComponent.Activate` (`self.LinesLeft`) false)
      (`ActorComponent.Activate` (`self.LinesBrake`) false))))

(fn `UserConstructionScript`)