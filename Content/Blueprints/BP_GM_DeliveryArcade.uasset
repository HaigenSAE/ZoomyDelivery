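; Game mode for a hoverbike delivery arcade game, running a countdown timer and tracking the current game state.
; BeginPlay resets the timer and initial state; StartTimer starts the countdown, enables hoverbike movement and advances the state.
; Tick decrements the timer and disables movement at zero, without changing state.
; UpdateState stores previous and current states, then fires the UpdatingState dispatcher.
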(event `self.ReceiveBeginPlay`
  (set `self.TimerCurrent` (`self.TimerStart`))
  (`self.UpdateState` "NewEnumerator0"))

(event `StartTimer`
  (set `self.TimerRunning` true)
  (set `/Game/Blueprints/Character/BP_Hoverbike.CanMove` true (cast `/Game/Blueprints/Character/BP_Hoverbike` (`GameplayStatics.GetPlayerPawn` 0) :!pure true))
  (`self.UpdateState` "NewEnumerator1"))

(event `self.ReceiveTick`
  (params (DeltaSeconds :type "Float (single-precision)"))
  (if (<= (`self.TimerCurrent`) 0.0)
    (bind _asbp_hoverbike (cast `/Game/Blueprints/Character/BP_Hoverbike` (`GameplayStatics.GetPlayerPawn` 0)))
    (set `/Game/Blueprints/Character/BP_Hoverbike.CanMove` false _asbp_hoverbike)
    (elif (`self.TimerRunning`)
      (set `self.TimerCurrent` (- (`self.TimerCurrent`) (`GameplayStatics.GetWorldDeltaSeconds`))))))

(fn `UpdateState`
  (params (NewState :type "/Game/Blueprints/Enum_GameState Enum" :default "NewEnumerator0"))
  (set `self.PreviousState` (`self.CurrentState`))
  (set `self.CurrentState` NewState)
  (`self.UpdatingState`))

(fn `UserConstructionScript`)