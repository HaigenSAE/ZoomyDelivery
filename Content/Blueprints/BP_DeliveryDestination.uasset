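; Delivery drop-off point with an NPC for an arcade delivery game, completed when the hoverbike enters its sphere while active.
; Activate and Deactivate toggle the NPC's waiting animation, the ring marker's visibility and the sphere's overlap detection.
; The overlap sets the game mode to Pickup, which deactivates the destination through a bound state event, and drops the player's package at the delivery location.
; Tick pulses and spins the ring.
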(event `self.ReceiveBeginPlay`
  (add `/Game/Blueprints/BP_GM_DeliveryArcade.UpdatingState` (cast `/Game/Blueprints/BP_GM_DeliveryArcade` (`GameplayStatics.GetGameMode`) :!pure true) (delegate `UpdatingState`)))

(event `UpdatingState`
  (switch `/Game/Blueprints/Enum_GameState` (`/Game/Blueprints/BP_GM_DeliveryArcade.CurrentState` (cast `/Game/Blueprints/BP_GM_DeliveryArcade` (`GameplayStatics.GetGameMode`) :!pure true))
    (:`NewEnumerator1`
      (`self.Deactivate`))))

(event `self.ReceiveTick`
  (params (DeltaSeconds :type "Float (single-precision)"))
  (bind _returnvalue (`KismetMathLibrary.Lerp` (`self.MinShrink`) 5.75 (`KismetMathLibrary.MakePulsatingValue` (`KismetSystemLibrary.GetGameTimeInSeconds`) 0.5)))
  (`SceneComponent.SetRelativeScale3D` (`self.Ring`) (`KismetMathLibrary.MakeVector` _returnvalue _returnvalue))
  (`SceneComponent.K2_AddLocalRotation` (`self.Ring`) (struct :`Yaw` 1.0) false false))

(event `Activate`
  (bind _sphere (`self.Sphere`))
  (set `self.Active` true)
  (set `/Game/Meshes/AnimBP_NPC.WaitingForDelivery` true (cast `/Game/Meshes/AnimBP_NPC` (`SkeletalMeshComponent.GetAnimInstance` (`self.SkeletalMesh`)) :!pure true))
  (`SceneComponent.SetVisibility` (`self.Ring`) true false)
  (`PrimitiveComponent.SetCollisionEnabled` _sphere "QueryOnly")
  (set `PrimitiveComponent.bGenerateOverlapEvents` true _sphere))

(event `Deactivate`
  (bind _sphere (`self.Sphere`))
  (set `self.Active` false)
  (set `/Game/Meshes/AnimBP_NPC.WaitingForDelivery` false (cast `/Game/Meshes/AnimBP_NPC` (`SkeletalMeshComponent.GetAnimInstance` (`self.SkeletalMesh`)) :!pure true))
  (`SceneComponent.SetVisibility` (`self.Ring`) false false)
  (`PrimitiveComponent.SetCollisionEnabled` _sphere "NoCollision")
  (set `PrimitiveComponent.bGenerateOverlapEvents` false _sphere))

(event `self.Sphere.OnComponentBeginOverlap`
  (params (OverlappedComponent :type "PrimitiveComponent Object Reference") (OtherActor :type "Actor Object Reference") (OtherComp :type "PrimitiveComponent Object Reference") (OtherBodyIndex :type Integer) (bFromSweep :type Boolean) (SweepResult :type "HitResult Structure (by ref)"))
  (if (and (== (`GameplayStatics.GetObjectClass` OtherActor) "/Game/Blueprints/Character/BP_Hoverbike.BP_Hoverbike_C") (`self.Active`))
    (set `self.MinShrink` 0.0)
    (`/Game/Blueprints/BP_GM_DeliveryArcade.UpdateState` (cast `/Game/Blueprints/BP_GM_DeliveryArcade` (`GameplayStatics.GetGameMode`) :!pure true) "NewEnumerator1")
    (`/Game/Blueprints/Character/BP_Package.DropOff` (`/Game/Blueprints/Character/BP_Hoverbike.CurrentPackage` (cast `/Game/Blueprints/Character/BP_Hoverbike` (`GameplayStatics.GetPlayerPawn` 0) :!pure true)) (`self.DeliverLoc`))))

(fn `UserConstructionScript`)