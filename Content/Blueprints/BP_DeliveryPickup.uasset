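; Delivery pickup actor that shows a pulsing, spinning ring and removes itself after a hoverbike reaches it.
; Tick scales the flattened ring between MinShrink and a fixed maximum using a game-time pulse, and rotates it a fixed step per frame.
; A BP_Hoverbike overlapping the sphere zeroes MinShrink, so the pulse's next low point shrinks the ring below a threshold and destroys the actor.
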(event `self.ReceiveTick`
  (params (DeltaSeconds :type "Float (single-precision)"))
  (bind _returnvalue (`KismetMathLibrary.Lerp` (`self.MinShrink`) 5.75 (`KismetMathLibrary.MakePulsatingValue` (`KismetSystemLibrary.GetGameTimeInSeconds`) 0.5)))
  (`SceneComponent.SetRelativeScale3D` (`self.Ring`) (`KismetMathLibrary.MakeVector` _returnvalue _returnvalue))
  (`SceneComponent.K2_AddLocalRotation` (`self.Ring`) (struct :`Yaw` 1.0) false false)
  (if (<= (.x (`SceneComponent.RelativeScale3D` (`self.Ring`))) 0.1)
    (`self.K2_DestroyActor`)))

(event `self.Sphere.OnComponentBeginOverlap`
  (params (OverlappedComponent :type "PrimitiveComponent Object Reference") (OtherActor :type "Actor Object Reference") (OtherComp :type "PrimitiveComponent Object Reference") (OtherBodyIndex :type Integer) (bFromSweep :type Boolean) (SweepResult :type "HitResult Structure (by ref)"))
  (if (== (`GameplayStatics.GetObjectClass` OtherActor) "/Game/Blueprints/Character/BP_Hoverbike.BP_Hoverbike_C")
    (set `self.MinShrink` 0.0)))

(fn `UserConstructionScript`)