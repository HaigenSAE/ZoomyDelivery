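; Character select flight path that moves a camera between spline points to view each character in an array.
; Left and Right keys step a wrapping point index, return the current character to idle and tell the new one it is being viewed.
; A Fly timeline lerps the camera from its current transform to the spline point, rotating it to face that character, with point 15 mapped to character 0.
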(event `Key|Left`
  (params (Key :type "Key Structure"))
  (:`Pressed`
    (`self.MoveLeft`)))

(event `Key|Right`
  (params (Key :type "Key Structure"))
  (:`Pressed`
    (`self.MoveRight`)))

(event `MoveLeft`
  (bind _pointindex (`self.PointIndex`))
  (bind _pointindex_2 (`self.PointIndex`))
  (bind _camera (`self.Camera`))
  (bind _pointindex_3 (`self.PointIndex`))
  (bind _returnvalue (`SplineComponent.GetLocationAtSplinePoint` (`self.Spline`) (`self.PointIndex`) "World"))
  (`self.ReturnCharToIdle`)
  (set `self.PointIndex` (select `bool` (== _pointindex_2 0) :`false` (- _pointindex_2 1) :`true` 14))
  (`/Game/Blueprints/Enviro/BP_CharacterSelectAI.BeingViewed` (`|GetArrayItem` (`self.Characters`) (select `bool` (== _pointindex 15) :`false` _pointindex)) :!label _label)
  (bind (_direction _alpha) (`Timeline|Fly` :!via `PlayFromStart`)
    (:`Update`
      (`SceneComponent.K2_SetWorldLocationAndRotation` (`self.Camera`) (`KismetMathLibrary.VLerp` (`SceneComponent.K2_GetComponentLocation` _camera) _returnvalue _alpha) (`KismetMathLibrary.RLerp` (`SceneComponent.K2_GetComponentRotation` _camera) (`KismetMathLibrary.FindLookAtRotation` _returnvalue (`self.K2_GetActorLocation` (`|GetArrayItem` (`self.Characters`) (select `bool` (== _pointindex_3 15) :`false` _pointindex_3)))) _alpha true) false false))))

(event `MoveRight`
  (bind _pointindex (`self.PointIndex`))
  (`self.ReturnCharToIdle`)
  (set `self.PointIndex` (select `bool` (== _pointindex 15) :`false` (+ _pointindex 1) :`true` 1))
  (goto _label))

(fn `ReturnCharToIdle`
  (bind _pointindex (`self.PointIndex`))
  (`/Game/Blueprints/Enviro/BP_CharacterSelectAI.Idle` (`|GetArrayItem` (`self.Characters`) (select `bool` (== _pointindex 15) :`false` _pointindex))))

(fn `UserConstructionScript`)