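; Spline-based road actor that builds road meshes along its RoadTrack spline in the Construction Script, with no active runtime logic.
; It splits the spline length by Distance and adds a collision-enabled spline mesh per segment, using the spline's local locations and its directions scaled by Tangent.
; When DoubleWide is set, each segment gets a second spline mesh using StaticMeshFlip on the same start and end points.
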(fn `UserConstructionScript`
  (bind _roadtrack (`self.RoadTrack`))
  (bind _distance (`self.Distance`))
  (for _index (range (+ (`.ReturnValue` (`KismetMathLibrary.FMod` (`SplineComponent.GetSplineLength` (`self.RoadTrack`)) (`self.Distance`))) 1))
    (bind _returnvalue (`AddComponent|NODE_AddSplineMeshComponent-0`))
    (`PrimitiveComponent.SetCollisionEnabled` _returnvalue "QueryAndPhysics")
    (`StaticMeshComponent.SetStaticMesh` _returnvalue (`self.StaticMesh`))
    (bind _returnvalue_2 (* _index _distance))
    (bind _returnvalue_3 (`SplineComponent.GetLocationAtDistanceAlongSpline` _roadtrack _returnvalue_2 "Local"))
    (bind _returnvalue_4 (* (`SplineComponent.GetDirectionAtDistanceAlongSpline` _roadtrack _returnvalue_2 "Local") (`self.Tangent`)))
    (bind _returnvalue_5 (+ _returnvalue_2 _distance))
    (bind _returnvalue_6 (`SplineComponent.GetLocationAtDistanceAlongSpline` _roadtrack _returnvalue_5 "Local"))
    (bind _returnvalue_7 (* (`SplineComponent.GetDirectionAtDistanceAlongSpline` _roadtrack _returnvalue_5 "Local") (`self.Tangent`)))
    (`SplineMeshComponent.SetStartAndEnd` _returnvalue _returnvalue_3 _returnvalue_4 _returnvalue_6 _returnvalue_7 true)
    (if (`self.DoubleWide`)
      (bind _returnvalue_8 (`AddComponent|NODE_AddSplineMeshComponent-1`))
      (`PrimitiveComponent.SetCollisionEnabled` _returnvalue_8 "QueryAndPhysics")
      (`StaticMeshComponent.SetStaticMesh` _returnvalue_8 (`self.StaticMeshFlip`))
      (`SplineMeshComponent.SetStartAndEnd` _returnvalue_8 _returnvalue_3 _returnvalue_4 _returnvalue_6 _returnvalue_7 true))))