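; BP_FlyingCar is an environment flying car that travels along the spline of a referenced track actor.
; On BeginPlay, active cars run a timeline with play rate set by Duration and start position by StartOffset.
; Its alpha maps to distance along the spline, setting world location directly while rotation eases toward the spline's direction with RInterpTo.
; The construction script applies the chosen vehicle skeletal mesh.
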(event `self.ReceiveBeginPlay`
  (if (`self.ActiveCar`)
    (`self.MoveCar`)))

(event `MoveCar`
  (bind _returnvalue (`KismetMathLibrary.Lerp` 0.0 (`SplineComponent.GetSplineLength` (`/Game/Blueprints/Enviro/BP_FlightTrack.SplinePath` (`self.TrackRef`))) (`self.Alpha`)))
  (`TimelineComponent.SetPlayRate` (`self.FlightTimeline`) (/ 1.0 (`self.Duration`)))
  (`TimelineComponent.SetNewTime` (`self.FlightTimeline`) (`self.StartOffset`))
  (bind (_direction _alpha) (`Timeline|FlightTimeline`)
    (:`Update`
      (set `self.Alpha` _alpha)
      (`self.K2_SetActorLocationAndRotation` (`SplineComponent.GetLocationAtDistanceAlongSpline` (`/Game/Blueprints/Enviro/BP_FlightTrack.SplinePath` (`self.TrackRef`)) _returnvalue "World") (`KismetMathLibrary.RInterpTo` (`self.K2_GetActorRotation`) (`SplineComponent.GetRotationAtDistanceAlongSpline` (`/Game/Blueprints/Enviro/BP_FlightTrack.SplinePath` (`self.TrackRef`)) _returnvalue "World") (`GameplayStatics.GetWorldDeltaSeconds`) 10.0)))))

(fn `UserConstructionScript`
  (`SkinnedMeshComponent.SetSkinnedAssetAndUpdate` (`self.SK_Veh_Future_01`) (`self.VehicleMesh`) true))