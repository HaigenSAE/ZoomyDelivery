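; Ambient wandering NPC that gets a random cyberpunk character mesh on construction and a random walk speed at BeginPlay.
; WalkEvent loops AI moves to random navigable points with random pauses, driving the AnimBP_NPC walking flag.
; TalkingSphere overlaps roll for willingness to talk; if both NPCs are willing, BeginChat walks to the partner, faces it and sets the chat animation flag for a random time, retrying failed moves.
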(event `self.ReceiveBeginPlay`
  (bind _output_get (set `self.WalkSpeed` (`KismetMathLibrary.RandomFloatInRange` 100.0 200.0)))
  (set `CharacterMovementComponent.MaxWalkSpeed` _output_get (`self.CharacterMovement`))
  (`self.WalkEvent`))

(event `WalkEvent`
  (bind _output_get (set `/Game/Meshes/AnimBP_NPC.Walking` (`self.Walking`) (cast `/Game/Meshes/AnimBP_NPC` (`SkeletalMeshComponent.GetAnimInstance` (`self.Mesh`)) :!pure true)))
  (if (not (and _output_get (not (`self.Chatting`))))
    (`|AIMoveTo` self (`NavigationSystemV1.K2_GetRandomLocationInNavigableRadius` (`self.K2_GetActorLocation`) (`self.WalkRadius`) null null) null
      (:`then`
        (bind _output_get_2 (set `self.Walking` true))
        (set `/Game/Meshes/AnimBP_NPC.Walking` _output_get_2 (cast `/Game/Meshes/AnimBP_NPC` (`SkeletalMeshComponent.GetAnimInstance` (`self.Mesh`)) :!pure true)))
      (:`OnSuccess`
        (set `/Game/Meshes/AnimBP_NPC.Walking` false (cast `/Game/Meshes/AnimBP_NPC` (`SkeletalMeshComponent.GetAnimInstance` (`self.Mesh`)) :!pure true) :!label _label)
        (`KismetSystemLibrary.Delay` (`KismetMathLibrary.RandomFloatInRange` 5.0 20.0))
        (set `self.Walking` false)
        (`self.WalkEvent`))
      (:`OnFail`
        (goto _label)))))

(event `self.ReceiveTick`
  (params (DeltaSeconds :type "Float (single-precision)")))

(event `self.TalkingSphere.OnComponentBeginOverlap`
  (params (OverlappedComponent :type "PrimitiveComponent Object Reference") (OtherActor :type "Actor Object Reference") (OtherComp :type "PrimitiveComponent Object Reference") (OtherBodyIndex :type Integer) (bFromSweep :type Boolean) (SweepResult :type "HitResult Structure (by ref)"))
  (set `self.WantsToTalk` (select `int` (`KismetMathLibrary.RandomIntegerInRange` 0 5) :`0` true :`1` false :`2` false :`3` false :`4` false :`5` true))
  (if (and (== (`GameplayStatics.GetObjectClass` OtherActor) "BP_NPCAI_C") (not (`self.Chatting`)) (!= OtherActor self) (`self.WantsToTalk`))
    (if (`/Game/Blueprints/Enviro/BP_NPCAI.WantsToTalk` (cast `/Game/Blueprints/Enviro/BP_NPCAI` OtherActor :!pure true))
      (set `self.NPC_Chat` OtherActor)
      (`self.BeginChat`))))

(event `BeginChat`
  (bind _returnvalue (`self.K2_GetActorLocation` (`self.NPC_Chat`)))
  (`|AIMoveTo` self _returnvalue null
    (:`OnSuccess`
      (`self.K2_SetActorRotation` (`KismetMathLibrary.FindLookAtRotation` (`self.K2_GetActorLocation`) _returnvalue))
      (bind _output_get (set `self.Chatting` true))
      (set `/Game/Meshes/AnimBP_NPC.IsWithAnotherNPC` _output_get (cast `/Game/Meshes/AnimBP_NPC` (`SkeletalMeshComponent.GetAnimInstance` (`self.Mesh`)) :!pure true))
      (`KismetSystemLibrary.Delay` (`KismetMathLibrary.RandomFloatInRange` 10.0 30.0))
      (set `/Game/Meshes/AnimBP_NPC.IsWithAnotherNPC` false (cast `/Game/Meshes/AnimBP_NPC` (`SkeletalMeshComponent.GetAnimInstance` (`self.Mesh`)) :!pure true))
      (set `self.Chatting` false)
      (set `self.NPC_Chat` null))
    (:`OnFail`
      (`self.BeginChat`))))

(fn `UserConstructionScript`
  (`SkinnedMeshComponent.SetSkinnedAssetAndUpdate` (`self.Mesh`) (select `int` (`KismetMathLibrary.RandomIntegerInRange` 0 17) :`0` "/Game/PolygonScifi/Meshes/Characters/SK_Character_Alien_Male_01.SK_Character_Alien_Male_01" :`1` "/Game/PolygonScifi/Meshes/Characters/SK_Character_Alien_Male_02.SK_Character_Alien_Male_02" :`2` "/Game/PolygonScifi/Meshes/Characters/SK_Character_Android_Female_01.SK_Character_Android_Female_01" :`3` "/Game/PolygonScifi/Meshes/Characters/SK_Character_Augmented_Male_01.SK_Character_Augmented_Male_01" :`4` "/Game/PolygonScifi/Meshes/Characters/SK_Character_Cop_01.SK_Character_Cop_01" :`5` "/Game/PolygonScifi/Meshes/Characters/SK_Character_Cyber_Female_01.SK_Character_Cyber_Female_01" :`6` "/Game/PolygonScifi/Meshes/Characters/SK_Character_Cyber_Male_01.SK_Character_Cyber_Male_01" :`7` "/Game/PolygonScifi/Meshes/Characters/SK_Character_CyberPunk_Male_01.SK_Character_CyberPunk_Male_01" :`8` "/Game/PolygonScifi/Meshes/Characters/SK_Character_Garbage_Male_01.SK_Character_Garbage_Male_01" :`9` "/Game/PolygonScifi/Meshes/Characters/SK_Character_Hacker_Female_01.SK_Character_Hacker_Female_01" :`10` "/Game/PolygonScifi/Meshes/Characters/SK_Character_Junky_Female_01.SK_Character_Junky_Female_01" :`11` "/Game/PolygonScifi/Meshes/Characters/SK_Character_Junky_Male_01.SK_Character_Junky_Male_01" :`12` "/Game/PolygonScifi/Meshes/Characters/SK_Character_Medical_Male_01.SK_Character_Medical_Male_01" :`13` "/Game/PolygonScifi/Meshes/Characters/SK_Character_Monk_Male_01.SK_Character_Monk_Male_01" :`14` "/Game/PolygonScifi/Meshes/Characters/SK_Character_Muscle_Male_01.SK_Character_Muscle_Male_01" :`15` "/Game/PolygonScifi/Meshes/Characters/SK_Character_Rich_Female_01.SK_Character_Rich_Female_01" :`16` "/Game/PolygonScifi/Meshes/Characters/SK_Character_Alien_Male_01.SK_Character_Alien_Male_01" :`17` "/Game/PolygonScifi/Meshes/Characters/SK_Character_Robot_01.SK_Character_Robot_01" :!type "SkeletalMesh Object Reference") true))